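; BP_RoomManager builds GeoMaze's 3D maze of cube rooms: one correct path surrounded by death rooms.
; The construction script chains straight runs along three shuffled, randomly signed axis directions, then adds death cubes at unoccupied six-direction neighbours.
; CreateCube assembles each room from static meshes and a tagged collision box, sized and spaced using mesh bounds.
; BeginPlay registers the manager with GameMode and GameInstance, then calls CallCoordinatesGenerated.
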(event `self.ReceiveBeginPlay`
  (bind _asgm_geo_maze (cast `/Game/MinuSkriptid/GM_GeoMaze` (`GameplayStatics.GetGameMode`)))
  (set `/Game/MinuSkriptid/GM_GeoMaze.As BP_RoomManager` self _asgm_geo_maze)
  (bind _asgi_geo_maze (cast `/Game/MinuSkriptid/GI_GeoMaze` (`GameplayStatics.GetGameInstance`)))
  (bind _output_get (set `/Game/MinuSkriptid/GI_GeoMaze.BP_RoomManager` self _asgi_geo_maze))
  (`self.CoordinatesGenerated` _output_get))

(event `CollidesWithCorrectCollision`)

(event `CollidesWithDeathCollision`)

(fn `CreateCube`
  (params (VectorIn :type "Vector Structure") (`CorrectCube?` :type Boolean))
  (returns (VectorOut :type "Vector Structure"))
  (locals (VectorInOut :type "Vector Structure"))
  (bind _vectorinout (`local.VectorInOut`))
  (bind (_vectorinout_x _vectorinout_y _vectorinout_z) (`KismetMathLibrary.BreakVector` (`local.VectorInOut`)))
  (bind _output_get (set `local.VectorInOut` VectorIn))
  (bind _returnvalue (`AddComponent|NODE_AddStaticMeshComponent-0` :`RelativeTransform` (`KismetMathLibrary.MakeTransform` _output_get)))
  (`AddComponent|NODE_AddStaticMeshComponent-7` :`RelativeTransform` (`KismetMathLibrary.MakeTransform` _vectorinout))
  (`AddComponent|NODE_AddStaticMeshComponent-8` :`RelativeTransform` (`KismetMathLibrary.MakeTransform` _vectorinout (struct :`Yaw` -90.0)))
  (`AddComponent|NODE_AddStaticMeshComponent-9` :`RelativeTransform` (`KismetMathLibrary.MakeTransform` _vectorinout))
  (`AddComponent|NODE_AddStaticMeshComponent-1` :`RelativeTransform` (`KismetMathLibrary.MakeTransform` _vectorinout))
  (for _index (range 4)
    (bind _returnvalue_2 (`AddComponent|NODE_AddStaticMeshComponent-2` :`RelativeTransform` (`KismetMathLibrary.MakeTransform` _vectorinout (`KismetMathLibrary.MakeRotator` 0.0 0.0 (`KismetMathLibrary.Conv_IntToDouble` (* _index 90)))))))
  (bind _returnvalue_3 (`StaticMesh.GetBoundingBox` (`StaticMeshComponent.StaticMesh` _returnvalue_2)))
  (bind _returnvalue_4 (`StaticMesh.GetBoundingBox` (`StaticMeshComponent.StaticMesh` _returnvalue)))
  (`AddComponent|NODE_AddStaticMeshComponent-6` :`RelativeTransform` (`KismetMathLibrary.MakeTransform` (`KismetMathLibrary.MakeVector` _vectorinout_x _vectorinout_y (+ _vectorinout_z (+ (- (.z (`.Max` (break `Box` _returnvalue_3))) (.z (break `Box` _returnvalue_3))) (- (.z (`.Max` (break `Box` _returnvalue_4))) (.z (break `Box` _returnvalue_4))))))))
  ;[1 1 1] Create Collisions
  (bind _returnvalue_5 (`AddComponent|NODE_AddBoxComponent-0` :`RelativeTransform` (`KismetMathLibrary.MakeTransform` (+ (`local.VectorInOut`) (0.0 0.0 300.0)) (struct) (12.0 12.0 12.0))))
  (if `CorrectCube?`
    (set `ActorComponent.ComponentTags` (`self.CorrectCollisionsTags`) _returnvalue_5)
    (`KismetArrayLibrary.Array_Add` (`self.CorrectCollisionsArray`) _returnvalue_5)
    (set `self.CorrectCollisionLast` _returnvalue_5)
    (else
      (set `ActorComponent.ComponentTags` (`self.DeathCollisionsTags`) _returnvalue_5)
      (`KismetArrayLibrary.Array_Add` (`self.DeathCollisionsArray`) _returnvalue_5)))
  (return (`local.VectorInOut`)))

(fn `UnitVectors_6`
  (returns (UnitVectorsArray6 :type "Array of Vector Structure"))
  (bind _unitvectorarray6 (`self.UnitVectorArray6`))
  (for _array_element (`self.UnitVectorArray1`)
    (`KismetArrayLibrary.Array_Add` (`self.UnitVectorArray6`) _array_element))
  (for _array_element_2 (`self.UnitVectorArray2`)
    (`KismetArrayLibrary.Array_Add` (`self.UnitVectorArray6`) _array_element_2))
  (for _array_element_3 (`self.UnitVectorArray3`)
    (`KismetArrayLibrary.Array_Add` _unitvectorarray6 _array_element_3))
  (return _unitvectorarray6))

(fn `UserConstructionScript`
  (bind (_stepxyz_x _stepxyz_y _stepxyz_z) (`KismetMathLibrary.BreakVector` (`self.StepXYZ`)))
  (bind _unitvectorarray (`self.UnitVectorArray`))
  (bind (_stepxyz_x_2 _stepxyz_y_2 _stepxyz_z_2) (`KismetMathLibrary.BreakVector` (`self.StepXYZ`)))
  (bind (_currentposition_x _currentposition_y _currentposition_z) (`KismetMathLibrary.BreakVector` (`self.CurrentPosition`)))
  (bind _returnvalue (`StaticMesh.GetBoundingBox` (`self.Wall`)))
  (bind _returnvalue_2 (`StaticMesh.GetBoundingBox` (`self.Floor`)))
  (bind _returnvalue_3 (- (.x (`.Max` (break `Box` _returnvalue_2))) (.x (break `Box` _returnvalue_2))))
  (`|ExecutionSequence`
    (:`then_0`
      ;[1 1 1] Õigete kuupide loomine
      (set `self.StepXYZ` (`KismetMathLibrary.MakeVector` _returnvalue_3 _returnvalue_3 (+ (* (- (.z (`.Max` (break `Box` _returnvalue_2))) (.z (break `Box` _returnvalue_2))) 2.0) (- (.z (`.Max` (break `Box` _returnvalue))) (.z (break `Box` _returnvalue))))))
      (bind _vectorout (`self.CreateCube` (0.0 0.0 0.0) true))
      (bind _output_get (set `self.CurrentPosition` _vectorout))
      (`KismetArrayLibrary.Array_Add` (`self.CorrectCubeLocations`) _output_get)
      ;;[1 1 1] Ruumide liikumissuundade järjekord
      (`KismetArrayLibrary.Array_Add` _unitvectorarray (`KismetArrayLibrary.Array_Random` (`self.UnitVectorArray1`)))
      (`KismetArrayLibrary.Array_Add` _unitvectorarray (`KismetArrayLibrary.Array_Random` (`self.UnitVectorArray2`)))
      (`KismetArrayLibrary.Array_Add` _unitvectorarray (`KismetArrayLibrary.Array_Random` (`self.UnitVectorArray3`)))
      (`KismetArrayLibrary.Array_Shuffle` _unitvectorarray)
      (for _array_element _unitvectorarray
        (for _ (range (+ (- (`self.TotalCubesInRow`) 2) 1))
          (bind _vectorout_2 (`self.CreateCube` (`KismetMathLibrary.MakeVector` (+ (* (.x _array_element) _stepxyz_x_2) _currentposition_x) (+ (* (.y _array_element) _stepxyz_y_2) _currentposition_y) (+ (* (.z _array_element) _stepxyz_z_2) _currentposition_z)) true))
          (bind _output_get_2 (set `self.CurrentPosition` _vectorout_2))
          (`KismetArrayLibrary.Array_Add` (`self.CorrectCubeLocations`) _output_get_2))))
    (:`then_1`
      ;[1 1 1] Create Death Cubes
      (bind _unitvectorsarray6 (`self.UnitVectors_6`))
      (for _array_element_2 (`self.CorrectCubeLocations`)
        (for _array_element_3 _unitvectorsarray6
          (bind _returnvalue_4 (`KismetMathLibrary.MakeVector` (+ (* (.x _array_element_3) _stepxyz_x) (.x _array_element_2)) (+ (* (.y _array_element_3) _stepxyz_y) (.y _array_element_2)) (+ (* (.z _array_element_3) _stepxyz_z) (.z _array_element_2))))
          (if (`KismetMathLibrary.BooleanNOR` (`KismetArrayLibrary.Array_Contains` (`self.CorrectCubeLocations`) _returnvalue_4) (`KismetArrayLibrary.Array_Contains` (`self.DeathCubeLocations`) _returnvalue_4))
            (bind _vectorout_3 (`self.CreateCube` _returnvalue_4))
            (`KismetArrayLibrary.Array_AddUnique` (`self.DeathCubeLocations`) _vectorout_3)))))
    (:`then_2`
      ;[1 1 1] Add all cubes to AllCubesLocations Array
      (for _array_element_4 (`self.CorrectCubeLocations`)
        (`KismetArrayLibrary.Array_AddUnique` (`self.AllCubesLocations`) _array_element_4))
      (for _array_element_5 (`self.DeathCubeLocations`)
        (`KismetArrayLibrary.Array_AddUnique` (`self.AllCubesLocations`) _array_element_5)))))