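; BP_DoorManager spawns BP_Door actors for the GeoMaze rooms, using cube locations from the room manager held in the game instance.
; GenerateNeighboringDoors runs after BeginPlay and on CoordinatesGenerated, finding the room center nearest the player.
; A macro computes six step-offset neighbor locations for the game instance.
; Doors spawn at every cube location and door angle, not just neighbors, with box-position checks intended to remove duplicates.
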(event `self.ReceiveBeginPlay`
  (`KismetSystemLibrary.Delay` 1.0)
  (bind _asgi_geo_maze (cast `/Game/MinuSkriptid/GI_GeoMaze` (`GameplayStatics.GetGameInstance`))
    (:`then`
      (set `self.As GI Geo Maze` _asgi_geo_maze)
      (bind _output_get (set `self.As BP Room Manager` (`/Game/MinuSkriptid/GI_GeoMaze.BP_RoomManager` _asgi_geo_maze)))
      (add `/Game/MinuSkriptid/BP_RoomManager.CoordinatesGenerated` (`self.As BP Room Manager`) (delegate `GenerateNeighboringDoors`))
      (`KismetSystemLibrary.Delay` 0.2)
      (`self.GenerateNeighboringDoors`))
    (:`CastFailed`
      (`KismetSystemLibrary.PrintString` "Hello"))))

(event `GenerateNeighboringDoors`
  ;[1 1 1] Get nearest centerpoint from the Player
  (bind _asbp_third_person_character_geo_maze (cast `/Game/MinuSkriptid/BP_ThirdPersonCharacter_GeoMaze` (`GameplayStatics.GetPlayerCharacter` 0))
    (:`then`
      (bind _allcubeslocations (`/Game/MinuSkriptid/BP_RoomManager.AllCubesLocations` (stale `self.ReceiveBeginPlay` _output_get)))
      (bind _closest (`/Game/MinuSkriptid/FL_Geomaze.FindClosestVector` _allcubeslocations (`SceneComponent.K2_GetComponentLocation` (`Character.CapsuleComponent` _asbp_third_person_character_geo_maze))))
      (`|ExecutionSequence`
        (:`then_0`
          (bind _neighboringroomlocations (`self.NeighboringRoomLocations` (`self.As BP Room Manager`) _closest :!label _label)
            (:`Exec`
              (set `/Game/MinuSkriptid/GI_GeoMaze.NeighboringRoomLocations` _neighboringroomlocations (`self.As GI Geo Maze`)))))
        (:`then_1`
          (goto _label :!via `Loc2`))
        (:`then_2`
          (goto _label :!via `Loc3`))
        (:`then_3`
          (goto _label :!via `Loc4`))
        (:`then_4`
          (goto _label :!via `Loc5`))
        (:`then_5`
          (goto _label :!via `Loc6`))
        (:`then_6`
          (for _array_element _allcubeslocations
            (for _array_element_2 (`self.DoorAngles`)
              (bind _returnvalue (`|SpawnActorFromClass` "/Game/MinuSkriptid/BP_Door.BP_Door_C" (`KismetMathLibrary.MakeTransform` _array_element (`KismetMathLibrary.MakeRotator` 0.0 0.0 _array_element_2)) "Undefined" "OverrideRootScale" null null))
              (for _array_element_3 (`self.BP_Door_Array`)
                (if (== (`SceneComponent.K2_GetComponentLocation` (`/Game/MinuSkriptid/BP_Door.Box` _array_element_3)) (`SceneComponent.K2_GetComponentLocation` (`/Game/MinuSkriptid/BP_Door.Box` _returnvalue)) :`ErrorTolerance` 10.0)
                  (`self.K2_DestroyActor` _returnvalue)
                  (else
                    (`KismetArrayLibrary.Array_Add` (`self.BP_Door_Array`) _returnvalue)))))))))
    (:`CastFailed`
      (`KismetSystemLibrary.PrintString` "BP_ThirdPersonCharacter FAILED"))))

(fn `UserConstructionScript`)