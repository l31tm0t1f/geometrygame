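; Game mode for GeoMaze that handles scoring, feedback and the win state as the player hits correct or death collisions.
; BeginPlay creates the main UI, caches the game instance and binds to the character's overlap events.
; Tick accumulates elapsed time in the game instance; correct hits award a minimum plus a speed bonus, while death hits apply damage points and a warning.
; The room manager's last correct collision disables movement and shows the win menu.
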(event `self.ReceiveBeginPlay`
  (bind _returnvalue (`|CreateWidget` "/Game/UI/UI_Main.UI_Main_C" (`GameplayStatics.GetPlayerController` 0)))
  (set `self.As UI Main` _returnvalue)
  (bind _asbp_third_person_character_geo_maze (cast `/Game/MinuSkriptid/BP_ThirdPersonCharacter_GeoMaze` (`GameplayStatics.GetPlayerCharacter` 0)))
  (bind _output_get (set `self.As BP Third Person Character Geo Maze` _asbp_third_person_character_geo_maze))
  (add `/Game/MinuSkriptid/BP_ThirdPersonCharacter_GeoMaze.PlayerBeginOverlapCorrectCollision` _output_get (`|CreateDelegate` :!event `CollidesWithCorrectCollision`))
  (add `/Game/MinuSkriptid/BP_ThirdPersonCharacter_GeoMaze.PlayerBeginOverlapDeathCollision` (`self.As BP Third Person Character Geo Maze`) (`|CreateDelegate` :!event `CollidesWithDeathCollision`))
  ;[1 1 1] Check this part - should go to Level BP
  (bind _asgi_geo_maze (cast `/Game/MinuSkriptid/GI_GeoMaze` (`GameplayStatics.GetGameInstance`)))
  (set `self.As GI Geo Maze` _asgi_geo_maze)
  (`Widget.SetVisibility` (`/Game/UI/UI_PointsAdd.TextBlock_PointsAdd` (`/Game/UI/UI_Main.UI_PointsAdd` (`self.As UI Main`))) "Hidden")
  (`Widget.SetVisibility` (`/Game/UI/UI_PointsAdd.TextBlock_PlussSign` (`/Game/UI/UI_Main.UI_PointsAdd` (`self.As UI Main`))) "Hidden")
  (`Widget.SetVisibility` (`/Game/UI/UI_Main.UI_Minimap` (`self.As UI Main`)) "Visible"))

(event `CollidesWithCorrectCollision`
  (bind _as_gi_geo_maze (`self.As GI Geo Maze`))
  (bind _as_gi_geo_maze_2 (`self.As GI Geo Maze`))
  (bind _as_gi_geo_maze_3 (`self.As GI Geo Maze`))
  (bind _as_ui_main (`self.As UI Main`))
  (bind _pointsmin (`/Game/MinuSkriptid/GI_GeoMaze.PointsMin` _as_gi_geo_maze))
  (bind _elapsedtime (`/Game/MinuSkriptid/GI_GeoMaze.ElapsedTime` _as_gi_geo_maze))
  (bind _elapsedtime_0 (`/Game/MinuSkriptid/GI_GeoMaze.ElapsedTime_0` _as_gi_geo_maze))
  (bind _pointstotal (`/Game/MinuSkriptid/GI_GeoMaze.PointsTotal` _as_gi_geo_maze_3))
  (bind _ui_pointsadd (`/Game/UI/UI_Main.UI_PointsAdd` (`self.As UI Main`)))
  ;[1 1 1] Calculate Points
  (if (< _elapsedtime _elapsedtime_0)
    (bind _output_get (set `/Game/MinuSkriptid/GI_GeoMaze.PointsAdd` (`KismetMathLibrary.Conv_IntToDouble` (`KismetMathLibrary.Round` (+ (* (- _elapsedtime_0 _elapsedtime) 5.0) _pointsmin))) _as_gi_geo_maze_3))
    (set `/Game/MinuSkriptid/GI_GeoMaze.PointsTotal` (+ _output_get _pointstotal) (`self.As GI Geo Maze`))
    (else
      (bind _output_get_2 (set `/Game/MinuSkriptid/GI_GeoMaze.PointsAdd` _pointsmin _as_gi_geo_maze_3))
      (set `/Game/MinuSkriptid/GI_GeoMaze.PointsTotal` (+ _output_get_2 _pointstotal) _as_gi_geo_maze_2)))
  ;[1 1 1] Missing: Add points to UI
  (set `/Game/MinuSkriptid/GI_GeoMaze.ElapsedTime` 0.0 _as_gi_geo_maze_2)
  (`Widget.SetVisibility` (`/Game/UI/UI_PointsAdd.TextBlock_PointsAdd` _ui_pointsadd) "Visible")
  (`Widget.SetVisibility` (`/Game/UI/UI_PointsAdd.TextBlock_PlussSign` _ui_pointsadd) "Visible")
  (`KismetSystemLibrary.Delay` 2.0)
  (`Widget.SetVisibility` (`/Game/UI/UI_PointsAdd.TextBlock_PlussSign` _ui_pointsadd) "Hidden")
  (`Widget.SetVisibility` (`/Game/UI/UI_PointsAdd.TextBlock_PointsAdd` _ui_pointsadd) "Hidden")
  ;[1 1 1] If last Correct Cube (collision)
  (if (== (`/Game/MinuSkriptid/BP_ThirdPersonCharacter_GeoMaze.DestroyableCollision` (`self.As BP Third Person Character Geo Maze`)) (`/Game/MinuSkriptid/BP_RoomManager.CorrectCollisionLast` (`self.As BP_RoomManager`)))
    ;[1 1 1] Diseable movement, show cursor etc
    (bind _aspc_geo_maze (cast `/Game/MinuSkriptid/PC_GeoMaze` (`GameplayStatics.GetPlayerController` 0)))
    (`/Game/MinuSkriptid/PC_GeoMaze.Set Input Mode UI Only` _aspc_geo_maze)
    (set `PlayerController.bShowMouseCursor` true _aspc_geo_maze)
    (`CharacterMovementComponent.DisableMovement` (`Character.CharacterMovement` (`self.As BP Third Person Character Geo Maze`)))
    (`/Game/MinuSkriptid/FL_Geomaze.SetText` "You Won!!!")
    (`Widget.SetVisibility` (`/Game/UI/UI_Main.UI_MainMenu` _as_ui_main) "Visible")
    (`Widget.SetVisibility` (`/Game/UI/UI_Main.UI_Minimap` _as_ui_main) "Hidden")))

(event `CollidesWithDeathCollision`
  (bind _as_gi_geo_maze (`self.As GI Geo Maze`))
  (bind _textblock_pointsadd (`/Game/UI/UI_PointsAdd.TextBlock_PointsAdd` (`/Game/UI/UI_Main.UI_PointsAdd` (`self.As UI Main`))))
  ;[1 1 1] Reduce Points
  (bind _output_get (set `/Game/MinuSkriptid/GI_GeoMaze.PointsAdd` (`self.PointsDamage`) _as_gi_geo_maze))
  (set `/Game/MinuSkriptid/GI_GeoMaze.PointsTotal` (+ _output_get (`/Game/MinuSkriptid/GI_GeoMaze.PointsTotal` _as_gi_geo_maze)) _as_gi_geo_maze)
  ;[1 1 1] Show Reduced points
  (`Widget.SetVisibility` _textblock_pointsadd "Visible")
  (`KismetSystemLibrary.Delay` 2.0)
  (`Widget.SetVisibility` _textblock_pointsadd "Hidden")
  ;[1 1 1] Show Damage Text
  (`/Game/MinuSkriptid/FL_Geomaze.SetText` "WRONG ROOM! DAMAGE!!!")
  (`KismetSystemLibrary.Delay` 3.0)
  (`/Game/MinuSkriptid/FL_Geomaze.SetText` ""))

(event `self.ReceiveTick`
  (params (DeltaSeconds :type "Float (single-precision)"))
  (bind _as_gi_geo_maze (`self.As GI Geo Maze`))
  ;[1 1 1] Count Seconds
  ;;[1 1 1] ERROR
  (set `/Game/MinuSkriptid/GI_GeoMaze.ElapsedTime` (+ DeltaSeconds (`/Game/MinuSkriptid/GI_GeoMaze.ElapsedTime` _as_gi_geo_maze)) _as_gi_geo_maze))

(fn `UserConstructionScript`)