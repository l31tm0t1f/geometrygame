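; Rising-platform actor for the GeoMaze game that carries the player up or down one room step at a time.
; After BeginPlay, it builds a 3D grid of mesh components with tagged trigger boxes, sized from the room manager's row count and step.
; Player overlap events and the Up/Down widget drive it, toggling input and menu visibility.
; Timelines lerp the whole actor vertically, with a DoOnce gate reset on end overlap.
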(event `self.ReceiveBeginPlay`
  (`KismetSystemLibrary.Delay` 0.2)
  (bind _asgm_geo_maze (cast `/Game/MinuSkriptid/GM_GeoMaze` (`GameplayStatics.GetGameMode`)))
  (bind _output_get (set `self.As GM Geo Maze` _asgm_geo_maze))
  (bind _output_get_2 (set `self.BP Room Manager` (`/Game/MinuSkriptid/GM_GeoMaze.As BP_RoomManager` _output_get)))
  (add `/Game/MinuSkriptid/BP_RoomManager.CoordinatesGenerated` _output_get_2 (`|CreateDelegate` :!event `CreateAllPlatforms`))
  (`self.CreateAllPlatforms`)
  (bind _asbp_third_person_character_geo_maze (cast `/Game/MinuSkriptid/BP_ThirdPersonCharacter_GeoMaze` (`GameplayStatics.GetPlayerCharacter` 0)))
  (bind _output_get_3 (set `self.As BP Third Person Character Geo Maze` _asbp_third_person_character_geo_maze))
  (add `/Game/MinuSkriptid/BP_ThirdPersonCharacter_GeoMaze.PlayerBeginOverlapPlatform` _output_get_3 (`|CreateDelegate` :!event `ShowUpDownUI`))
  (add `/Game/MinuSkriptid/BP_ThirdPersonCharacter_GeoMaze.PlayerEndOverlapPlatform` _output_get_3 (`|CreateDelegate` :!event `EndOverlap`))
  (bind _asgm_geo_maze_2 (cast `/Game/MinuSkriptid/GM_GeoMaze` (`GameplayStatics.GetGameMode`)))
  ;[1 1 1] ERROR
  (add `/Game/UI/UI_UpDown.UpOrDown` (`/Game/UI/UI_Main.UI_UpDown` (`/Game/MinuSkriptid/GM_GeoMaze.As UI Main` _asgm_geo_maze_2)) (`|CreateDelegate` :!event `GoesUpOrDown`)))

(event `CreateAllPlatforms`
  (bind _bp_room_manager (`self.BP Room Manager`))
  (bind (_firstplatformlocation_x _firstplatformlocation_y _firstplatformlocation_z) (`KismetMathLibrary.BreakVector` (`self.FirstPlatformLocation`)))
  (bind (_firstplatformlocation_x_2 _firstplatformlocation_y_2) (`KismetMathLibrary.BreakVector` (`self.FirstPlatformLocation`)))
  (bind _totalcubesinrow (`/Game/MinuSkriptid/BP_RoomManager.TotalCubesInRow` _bp_room_manager))
  (bind (_stepxyz_x _stepxyz_y _stepxyz_z) (`KismetMathLibrary.BreakVector` (`/Game/MinuSkriptid/BP_RoomManager.StepXYZ` _bp_room_manager)))
  (bind _returnvalue (* _totalcubesinrow 2))
  ;[1 1 1] Create Platforms
  (bind _output_get (set `self.FirstPlatformLocation` (`KismetMathLibrary.MakeVector` (* _totalcubesinrow _stepxyz_x -1) (* _totalcubesinrow _stepxyz_y -1) (* _stepxyz_z -1))))
  ;;[1 1 1] Platform X-direction
  (for _index (range (+ _returnvalue 1))
    (bind _output_get_2 (set `self.CurrentPlatformLocation` (`KismetMathLibrary.MakeVector` (+ (.x _output_get) (* _index _stepxyz_x)) (.y _output_get) (.z _output_get))))
    (`self.CreatePlatformWCollision` (`KismetMathLibrary.MakeVector` (.x _output_get_2) (.y _output_get_2) (.z _output_get_2)))
    ;;[1 1 1] Platform Y-direction
    (for _index_2 (range (+ _returnvalue 1))
      (bind _output_get_3 (set `self.CurrentPlatformLocation` (`KismetMathLibrary.MakeVector` (.x _output_get_2) (+ _firstplatformlocation_y_2 (* _index_2 _stepxyz_y)) (.z _output_get_2))))
      (`self.CreatePlatformWCollision` (`KismetMathLibrary.MakeVector` (.x _output_get_3) (.y _output_get_3) (.z _output_get_3)))
      ;;[1 1 1] Platform Z-direction
      (for _index_3 (range (+ _returnvalue 1))
        (bind _output_get_4 (set `self.CurrentPlatformLocation` (`KismetMathLibrary.MakeVector` (.x _output_get_3) (.y _output_get_3) (+ _firstplatformlocation_z (* _index_3 _stepxyz_z)))))
        (`self.CreatePlatformWCollision` _output_get_4)))))

(event `GoesUpOrDown`
  (params (IsUp :type Boolean))
  (bind _currentlocation (`self.CurrentLocation`))
  (bind _x (.x _currentlocation))
  (bind _y (.y _currentlocation))
  (bind _z (.z _currentlocation))
  (bind (_stepxyz_x _stepxyz_y _stepxyz_z) (`KismetMathLibrary.BreakVector` (`/Game/MinuSkriptid/BP_RoomManager.StepXYZ` (`self.BP Room Manager`))))
  ;[1 1 1] Up-Down Movement
  (set `self.CurrentLocation` (`self.K2_GetActorLocation`))
  (`/Engine/EditorBlueprintResources/StandardMacros.DoOnce` false :!label _label
    (:`Completed`
      (if IsUp
        (bind (_direction _newtrack_0) (`Timeline|Timeline_0` :!via `PlayFromStart`)
          (:`Update`
            (bind _returnvalue (`KismetMathLibrary.VLerp` _currentlocation (`KismetMathLibrary.MakeVector` _x _y (+ _z _stepxyz_z)) _newtrack_0))
            (`self.K2_SetActorLocation` _returnvalue true)
            (`Widget.SetVisibility` (`/Game/UI/UI_Main.UI_UpDown` (`/Game/MinuSkriptid/GM_GeoMaze.As UI Main` (`self.As GM Geo Maze`))) "Hidden" :!label _label_2))
          (:`Finished`
            (set `self.CurrentLocation` _returnvalue)))
        (else
          (bind (_direction_2 _newtrack_0_2) (`Timeline|Timeline` :!via `PlayFromStart`)
            (:`Update`
              (bind _returnvalue_2 (`KismetMathLibrary.VLerp` _currentlocation (`KismetMathLibrary.MakeVector` _x _y (- _z _stepxyz_z)) _newtrack_0_2))
              (`self.K2_SetActorLocation` _returnvalue_2 true)
              (goto _label_2))
            (:`Finished`
              (set `self.CurrentLocation` _returnvalue_2))))))))

(event `EndOverlap`
  ;[1 1 1] Up-Down Movement
  (`/Game/MinuSkriptid/FL_Geomaze.InputAndMovement` true)
  (goto _label :!via `Reset`))

(event `ShowUpDownUI`
  ;[1 1 1] Open Up-Down Menu, Disable Outputs etc
  (bind _asgm_geo_maze (cast `/Game/MinuSkriptid/GM_GeoMaze` (`GameplayStatics.GetGameMode`)))
  (`Widget.SetVisibility` (`/Game/UI/UI_Main.UI_UpDown` (`/Game/MinuSkriptid/GM_GeoMaze.As UI Main` _asgm_geo_maze)) "Visible")
  (`/Game/MinuSkriptid/FL_Geomaze.InputAndMovement` false))

(fn `CreatePlatformWCollision`
  (params (VectorLocation :type "Vector Structure"))
  ;[1 1 1] Create Platform + Collision
  (bind _returnvalue (`AddComponent|NODE_AddStaticMeshComponent-0` :`RelativeTransform` (`KismetMathLibrary.MakeTransform` VectorLocation)))
  (`StaticMeshComponent.SetStaticMesh` _returnvalue "/Game/RAW/Cube_parts_Mesh3.Cube_parts_Mesh3")
  (bind _returnvalue_2 (`AddComponent|NODE_AddBoxComponent-0` :`RelativeTransform` (`KismetMathLibrary.MakeTransform` VectorLocation (struct) (0.05 0.05 3.0))))
  (set `ActorComponent.ComponentTags` (`self.TagArray`) _returnvalue_2))

(fn `UserConstructionScript`)