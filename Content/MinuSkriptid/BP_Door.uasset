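; Door actor that slides up when the GeoMaze third-person character enters its box trigger and lowers when they leave.
; BeginPlay stores the closed relative location and measures the mesh's bounding-box height as travel distance.
; The DoorOpenClose timeline lerps between closed and raised positions, always restarting from either end.
; Leaving the trigger also calls DoorCloses before reversing the timeline.
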(event `self.ReceiveBeginPlay`
  (bind _door (`self.Door`))
  (bind _returnvalue (`StaticMesh.GetBoundingBox` (`StaticMeshComponent.StaticMesh` _door)))
  ;[1 1 1] Get/Set Door Height (how much should it move
  (set `self.HeightDoor` (- (.z (`.Max` (break `Box` _returnvalue))) (.z (break `Box` _returnvalue))))
  (set `self.RelativeLocation` (`SceneComponent.RelativeLocation` _door)))

(event `self.Box.OnComponentBeginOverlap`
  (params (OverlappedComponent :type "PrimitiveComponent Object Reference") (OtherActor :type "Actor Object Reference") (OtherComp :type "PrimitiveComponent Object Reference") (OtherBodyIndex :type Integer) (bFromSweep :type Boolean) (SweepResult :type "HitResult Structure (by ref)"))
  (bind _relativelocation (`self.RelativeLocation`))
  ;[1 1 1] Door Open/Close
  (cast `/Game/MinuSkriptid/BP_ThirdPersonCharacter_GeoMaze` OtherActor)
  (bind (_direction _newtrack_0) (`Timeline|DoorOpenClose` :!via `PlayFromStart` :!label _label)
    (:`Update`
      (`SceneComponent.K2_SetRelativeLocation` (`self.Door`) (`KismetMathLibrary.VLerp` _relativelocation (`KismetMathLibrary.MakeVector` (.x _relativelocation) (.y _relativelocation) (+ (.z _relativelocation) (`self.HeightDoor`))) _newtrack_0) false false))))

(event `self.Box.OnComponentEndOverlap`
  (params (OverlappedComponent :type "PrimitiveComponent Object Reference") (OtherActor :type "Actor Object Reference") (OtherComp :type "PrimitiveComponent Object Reference") (OtherBodyIndex :type Integer))
  ;[1 1 1] Door Open/Close
  (cast `/Game/MinuSkriptid/BP_ThirdPersonCharacter_GeoMaze` OtherActor)
  (`self.DoorCloses`)
  (goto _label :!via `ReverseFromEnd`))

(fn `UserConstructionScript`)