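; Collision manager for the GeoMaze game that spawns trigger volumes on maze cubes and handles reaching correct ones, including the win.
; At startup it adds tagged box components above the room manager's correct (except the first) and death cube locations.
; Player overlap delegates drive responses: correct hits show points, reset elapsed time and destroy the box.
; The last correct box triggers the win UI; the death handler is empty, pointing to GM_GeoMaze.
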(event `self.ReceiveBeginPlay`
  ;[1 1 1] Event Begin Play
  (`KismetSystemLibrary.Delay` 0.2)
  (bind _asgi_geo_maze (cast `/Game/MinuSkriptid/GI_GeoMaze` (`GameplayStatics.GetGameInstance`)))
  (set `self.As GI Geo Maze` _asgi_geo_maze)
  (bind _output_get (set `self.BP Room Manager` (`/Game/MinuSkriptid/GI_GeoMaze.BP_RoomManager` _asgi_geo_maze)))
  (add `/Game/MinuSkriptid/BP_RoomManager.CoordinatesGenerated` _output_get (`|CreateDelegate` :!event `CreateCollisions`))
  (`KismetSystemLibrary.Delay` 0.2)
  (`self.CreateCollisions`)
  (bind _asbp_third_person_character_geo_maze (cast `/Game/MinuSkriptid/BP_ThirdPersonCharacter_GeoMaze` (`GameplayStatics.GetPlayerCharacter` 0)))
  (add `/Game/MinuSkriptid/BP_ThirdPersonCharacter_GeoMaze.PlayerBeginOverlapCorrectCollision` _asbp_third_person_character_geo_maze (`|CreateDelegate` :!event `CollidesWithCorrectCollision`))
  (add `/Game/MinuSkriptid/BP_ThirdPersonCharacter_GeoMaze.PlayerBeginOverlapDeathCollision` _asbp_third_person_character_geo_maze (`|CreateDelegate` :!event `CollidesWithDeathCollision`)))

(event `CreateCollisions`
  (bind _correctcollisionarray (`self.CorrectCollisionArray`))
  (bind _bp_roommanager (`/Game/MinuSkriptid/GI_GeoMaze.BP_RoomManager` (stale `self.ReceiveBeginPlay` _asgi_geo_maze)))
  ;[1 1 1] Create Collisions
  ;;[1 1 1] Correct Collisions
  (for (_array_element _array_index) (`/Game/MinuSkriptid/BP_RoomManager.CorrectCubeLocations` _bp_roommanager)
    (if (!= _array_index 0)
      (bind _returnvalue (`AddComponent|NODE_AddBoxComponent-0` :`RelativeTransform` (`KismetMathLibrary.MakeTransform` (+ _array_element (0.0 0.0 300.0)) (struct) (12.0 12.0 12.0))))
      (set `ActorComponent.ComponentTags` (`self.CorrectCollisionTags`) _returnvalue)
      (`KismetArrayLibrary.Array_Add` (`self.CorrectCollisionArray`) _returnvalue)))
  (set `self.CorrectCollisionLast` (`|GetArrayItem` _correctcollisionarray (`KismetArrayLibrary.Array_LastIndex` _correctcollisionarray)))
  ;;[1 1 1] Death Collisions
  (for _array_element_2 (`/Game/MinuSkriptid/BP_RoomManager.DeathCubeLocations` _bp_roommanager)
    (bind _returnvalue_2 (`AddComponent|NODE_AddBoxComponent-1` :`RelativeTransform` (`KismetMathLibrary.MakeTransform` (+ _array_element_2 (0.0 0.0 300.0)) (struct) (12.0 12.0 12.0))))
    (set `ActorComponent.ComponentTags` (`self.DeathCollisionTags`) _returnvalue_2)
    (`KismetArrayLibrary.Array_Add` (`self.DeathCollisionArray`) _returnvalue_2)))

(event `CollidesWithCorrectCollision`
  (bind _returnvalue (`GameplayStatics.GetPlayerController` 0))
  ;[1 1 1] Make Widget Visible
  (bind _asgm_geo_maze (cast `/Game/MinuSkriptid/GM_GeoMaze` (`GameplayStatics.GetGameMode`)))
  (`Widget.SetVisibility` (`/Game/MinuSkriptid/UI_Main.UI_PointsAdd` (`/Game/MinuSkriptid/GM_GeoMaze.As UI_Main` _asgm_geo_maze)) "Visible")
  (set `/Game/MinuSkriptid/GI_GeoMaze.ElapsedTime` 0.0 (`self.As GI Geo Maze`))
  ;[1 1 1] Destroy Collision
  (bind _asbp_third_person_character_geo_maze (cast `/Game/MinuSkriptid/BP_ThirdPersonCharacter_GeoMaze` (`GameplayStatics.GetPlayerCharacter` 0)))
  (bind _output_get (set `self.Destroyable Collision` (`/Game/MinuSkriptid/BP_ThirdPersonCharacter_GeoMaze.DestroyableCollision` _asbp_third_person_character_geo_maze)))
  (`ActorComponent.K2_DestroyComponent` _output_get)
  ;[1 1 1] Last Collision - Winning Condition
  (if (== (`self.Destroyable Collision`) (`self.CorrectCollisionLast`))
    (`/Game/MinuSkriptid/FL_Geomaze.InputAndMovement` false)
    (bind _asgm_geo_maze_2 (cast `/Game/MinuSkriptid/GM_GeoMaze` (`GameplayStatics.GetGameMode`)))
    (`WidgetBlueprintLibrary.SetInputMode_UIOnlyEx` _returnvalue null)
    (set `PlayerController.bShowMouseCursor` true _returnvalue)
    (bind _ui_text (`/Game/MinuSkriptid/UI_Main.UI_Text` (`/Game/MinuSkriptid/GM_GeoMaze.As UI_Main` _asgm_geo_maze_2)))
    (set `/Game/MinuSkriptid/UI_Text.TextTextText` "You Won" _ui_text)
    (`Widget.SetVisibility` _ui_text "Visible")
    (`Widget.SetVisibility` (`/Game/MinuSkriptid/UI_Main.UI_RestartContinue` (`/Game/MinuSkriptid/GM_GeoMaze.As UI_Main` _asgm_geo_maze_2)) "Visible")
    (`KismetSystemLibrary.Delay` 3.0)
    (`Widget.SetVisibility` _ui_text "Hidden")
    (`Widget.SetVisibility` (`/Game/MinuSkriptid/UI_Main.UI_RestartContinue` (`/Game/MinuSkriptid/GM_GeoMaze.As UI_Main` _asgm_geo_maze_2)) "Hidden")))

(event `CollidesWithDeathCollision`
  ;[1 1 1] Check GM_GeoMaze
)

(fn `UserConstructionScript`)